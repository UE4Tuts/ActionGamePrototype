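; Animation modifier that bakes the root bone's yaw progress into a "RotationCurve" on the animation sequence.
; On apply, it adds the curve as a metadata curve, then writes a float key at each frame's time.
; Each key is that frame's root-motion yaw, remapped with clamping from the zero-to-final-frame yaw range into a normalized 0–1 value.
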(event `self.OnApply`
  (params (AnimationSequence :type "AnimSequence Object Reference"))
  (bind (_pose_location _pose_rotation) (`KismetMathLibrary.BreakTransform` (`AnimationBlueprintLibrary.GetBonePoseForFrame` (`self.AnimSeq`) "root" (`AnimationBlueprintLibrary.GetNumFrames` (`self.AnimSeq`)) true)))
  (set `self.AnimSeq` AnimationSequence)
  (`AnimationBlueprintLibrary.AddCurve` (`self.AnimSeq`) "RotationCurve" "RCT_Float" true)
  (for _index (range (+ (`AnimationBlueprintLibrary.GetNumFrames` (`self.AnimSeq`)) 1))
    (bind (_pose_location_2 _pose_rotation_2) (`KismetMathLibrary.BreakTransform` (`AnimationBlueprintLibrary.GetBonePoseForFrame` (`self.AnimSeq`) "root" _index true)))
    (`AnimationBlueprintLibrary.AddFloatCurveKey` (`self.AnimSeq`) "RotationCurve" (`AnimationBlueprintLibrary.GetTimeAtFrame` (`self.AnimSeq`) _index) (`KismetMathLibrary.MapRangeClamped` (.yaw _pose_rotation_2) 0.0 (.yaw _pose_rotation) 0.0 1.0))))