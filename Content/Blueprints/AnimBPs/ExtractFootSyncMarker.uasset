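; Animation modifier that automatically places foot_r and foot_l sync markers on a FootSyncMarkers notify track in an animation sequence.
; For each frame, it composes bone poses from each foot up to, but excluding, root to get the foot's height.
; When that height drops below a fixed threshold, a DoOnce gate limits markers to one per contact, resetting once the foot rises.
; Reverting removes the track.
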(event `self.OnApply`
  (params (AnimationSequence :type "AnimSequence Object Reference"))
  (bind _output_get (set `self.AnimSeq` AnimationSequence))
  (`AnimationBlueprintLibrary.AddAnimationNotifyTrack` _output_get "FootSyncMarkers" (struct :`R` 0.227848 :`G` 0.625 :`B` 0.214844 :`A` 1.0))
  (`|ExecutionSequence`
    (:`then_0`
      (for _index (range (+ (`AnimationBlueprintLibrary.GetNumFrames` (`self.AnimSeq`)) 1))
        (set `self.Index` _index)
        (set `self.Transform` (`KismetMathLibrary.MakeTransform` (0.0 0.0 0.0)))
        (for _array_element (`AnimationBlueprintLibrary.FindBonePathToRoot` (`self.AnimSeq`) "foot_r")
          (if (== _array_element "root")
            (break)
            (else
              (bind _output_get_2 (set `self.Transform` (`KismetMathLibrary.ComposeTransforms` (`self.Transform`) (`AnimationBlueprintLibrary.GetBonePoseForFrame` (`self.AnimSeq`) _array_element (`self.Index`))))))))
        (if (< (.z (.location _output_get_2)) 10.0)
          (`/Engine/EditorBlueprintResources/StandardMacros.DoOnce` true :!label _label
            (:`Completed`
              (`AnimationBlueprintLibrary.AddAnimationSyncMarker` (`self.AnimSeq`) "foot_r" (`AnimationBlueprintLibrary.GetTimeAtFrame` (`self.AnimSeq`) (`self.Index`)) "FootSyncMarkers")))
          (else
            (goto _label :!via `Reset`)))))
    (:`then_1`
      (for _index_2 (range (+ (`AnimationBlueprintLibrary.GetNumFrames` (`self.AnimSeq`)) 1))
        (set `self.Index` _index_2)
        (set `self.Transform` (`KismetMathLibrary.MakeTransform` (0.0 0.0 0.0)))
        (for _array_element_2 (`AnimationBlueprintLibrary.FindBonePathToRoot` (`self.AnimSeq`) "foot_l")
          (if (== _array_element_2 "root")
            (break)
            (else
              (bind _output_get_3 (set `self.Transform` (`KismetMathLibrary.ComposeTransforms` (`self.Transform`) (`AnimationBlueprintLibrary.GetBonePoseForFrame` (`self.AnimSeq`) _array_element_2 (`self.Index`))))))))
        (if (< (.z (.location _output_get_3)) 10.0)
          (`/Engine/EditorBlueprintResources/StandardMacros.DoOnce` true :!label _label_2
            (:`Completed`
              (`AnimationBlueprintLibrary.AddAnimationSyncMarker` (`self.AnimSeq`) "foot_l" (`AnimationBlueprintLibrary.GetTimeAtFrame` (`self.AnimSeq`) (`self.Index`)) "FootSyncMarkers")))
          (else
            (goto _label_2 :!via `Reset`)))))))

(event `self.OnRevert`
  (params (AnimationSequence :type "AnimSequence Object Reference"))
  (`AnimationBlueprintLibrary.RemoveAnimationNotifyTrack` AnimationSequence "FootSyncMarkers"))