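; Player camera manager that drives a third-person, over-the-shoulder follow camera for BP_PlayerCharacter.
; BlueprintUpdateCamera places the camera behind, right of and above the character with a fixed FOV, using an interpolated distance and rotation.
; Distance eases between running and idle targets based on whether movement acceleration is non-zero.
; Rotation eases toward player 0's control rotation, with a slower interp speed while accelerating.
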(event `OnPossess`
  (params (NewParam :type "Pawn Object Reference"))
  (set `self.ControlledPawn` NewParam))

(fn `BlueprintUpdateCamera`
  (params (CameraTarget :type "Actor Object Reference"))
  (returns (NewCameraLocation :type "Vector Structure") (NewCameraRotation :type "Rotator Structure") (NewCameraFOV :type "Float (single-precision)") (ReturnValue :type Boolean))
  (bind _targetcamerrotation (`self.TargetCamerRotation`))
  (bind _asbp_player_character (cast `/Game/Blueprints/BP_PlayerCharacter` CameraTarget))
  (set `self.Player` _asbp_player_character)
  (`self.Calculate Camera Distance`)
  (`self.CalculateCameraRotation`)
  (return (+ (`self.K2_GetActorLocation` (`self.Player`)) (+ (* (`KismetMathLibrary.GetForwardVector` _targetcamerrotation) (* (`self.TargetCameraDistance`) -1.0)) (* (`KismetMathLibrary.GetRightVector` _targetcamerrotation) 50.0)) (0.0 0.0 50.0)) (`self.TargetCamerRotation`) 85.0 true))

(fn `Calculate Camera Distance`
  (if (> (`KismetMathLibrary.VSize` (`CharacterMovementComponent.GetCurrentAcceleration` (`Character.CharacterMovement` (`self.Player`)))) 0.0)
    (bind _output_get (set `self.CameraDistanceInterp` (`KismetMathLibrary.FInterpTo` (stale _output_get) (`self.RunningCameraDistance`) (`GameplayStatics.GetWorldDeltaSeconds`) (`self.CameraInterpSpeed_Running`))))
    (else
      (bind _output_get_2 (set `self.CameraDistanceInterp` (`KismetMathLibrary.FInterpTo` (stale _output_get_2) (`self.IdleCameraDistance`) (`GameplayStatics.GetWorldDeltaSeconds`) (`self.CameraInterpSpeed_Idle`))))))
  (set `self.TargetCameraDistance` (`self.CameraDistanceInterp`))
  (return))

(fn `CalculateCameraRotation`
  (locals (InterpSpeed :type "Float (single-precision)" :default 15.0))
  (if (> (`KismetMathLibrary.VSize` (`CharacterMovementComponent.GetCurrentAcceleration` (`Character.CharacterMovement` (`self.Player`)))) 0.0)
    (set `local.InterpSpeed` 15.0)
    (else
      (set `local.InterpSpeed` 30.0)))
  (set `self.TargetCamerRotation` (`KismetMathLibrary.RInterpTo` (`self.GetCameraRotation`) (`Controller.GetControlRotation` (`GameplayStatics.GetPlayerController` 0)) (`GameplayStatics.GetWorldDeltaSeconds`) (`local.InterpSpeed`))))

(fn `UserConstructionScript`)